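; A potion collectible for the Kobo Dungeon level that reports itself to GM_BPCommunication, the game mode.
; It registers as a collectible one second after BeginPlay.
; When BP_Communications_Character overlaps its trigger, it hides the mesh and wisp effects, disables trigger collision, and notifies the game mode of the pickup.
; The actor is hidden rather than destroyed.
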(event `self.ReceiveBeginPlay`
  (`KismetSystemLibrary.Delay` 1.0)
  (bind _asgm_bpcommunication (cast `/Game/BPCommunication/Blueprints/GM_BPCommunication` (`GameplayStatics.GetGameMode`)))
  (`/Game/BPCommunication/Blueprints/GM_BPCommunication.CollectibleRegister` _asgm_bpcommunication))

(event `self.Trigger.OnComponentBeginOverlap`
  (params (OverlappedComponent :type "PrimitiveComponent Object Reference") (OtherActor :type "Actor Object Reference") (OtherComp :type "PrimitiveComponent Object Reference") (OtherBodyIndex :type Integer) (bFromSweep :type Boolean) (SweepResult :type "HitResult Structure (by ref)"))
  (cast `/Game/BPCommunication/Blueprints/BP_Communications_Character` OtherActor)
  (`SceneComponent.SetVisibility` (`self.SM-Potion-1`) false false)
  (`SceneComponent.SetVisibility` (`self.FX-PotionWhisps-01`) false false)
  (`SceneComponent.SetVisibility` (`self.FX-PotionWhisps-02`) false false)
  (`PrimitiveComponent.SetCollisionEnabled` (`self.Trigger`) "NoCollision")
  (bind _asgm_bpcommunication (cast `/Game/BPCommunication/Blueprints/GM_BPCommunication` (`GameplayStatics.GetGameMode`)))
  (`/Game/BPCommunication/Blueprints/GM_BPCommunication.CollectibleCollected` _asgm_bpcommunication))

(fn `UserConstructionScript`)