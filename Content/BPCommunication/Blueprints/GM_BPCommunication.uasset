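; GM_BPCommunication is a game mode Blueprint that tracks how many collectibles remain and shows the player UI.
; CollectibleRegister and CollectibleCollected increment and decrement CollectiblesLeft, then broadcast the new count through the OnCollectable dispatcher.
; On BeginPlay it binds its own listener, which prints the count, and adds UMG_PlayerUI to the viewport.
; Disconnected GetActorOfClass, OpenDoor and other actor-lookup nodes remain in the graph but never run.
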(event `self.ReceiveBeginPlay`
  (add `self.OnCollectable` (delegate `OnColection_Event`))
  (bind _returnvalue (`|CreateWidget` "/Game/BPCommunication/UMG/UMG_PlayerUI.UMG_PlayerUI_C"))
  (`UserWidget.AddToViewport` _returnvalue 0))

(event `OnColection_Event` :!signature `self.OnCollectable`
  (params (Cantidad :type Integer))
  (`KismetSystemLibrary.PrintText` (`KismetTextLibrary.Conv_IntToText` Cantidad)))

(event `CollectibleRegister`
  (bind _result (`/Engine/EditorBlueprintResources/StandardMacros.IncrementInt` (`self.CollectiblesLeft`))
    (:`  `
      (`self.OnCollectable` _result))))

(event `CollectibleCollected`
  (bind _result (`/Engine/EditorBlueprintResources/StandardMacros.DecrementInt` (`self.CollectiblesLeft`))
    (:`  `
      (`self.OnCollectable` _result))))

(fn `UserConstructionScript`)